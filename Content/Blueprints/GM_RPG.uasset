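; RPG game mode that puts the HUD widget on screen at BeginPlay and manages background music.
; UpdateBackgroundMusic treats BackgroundMusicColls as a priority stack: the last entry's sound plays, switching only if it differs, and an empty list stops the music.
; PlayMusic stops and destroys the current audio component, then creates and plays a new 2D sound.
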(event `self.ReceiveBeginPlay`
  (bind _returnvalue (`|CreateWidget` "/Game/Widgets/WBP_HUD.WBP_HUD_C"))
  (bind _output_get (set `self.HUDWidget` _returnvalue))
  (`UserWidget.AddToViewport` _output_get 0))

(event `PlayMusic`
  (params (Sound :type "SoundBase Object Reference"))
  (`|ExecutionSequence`
    (:`then_0`
      (bind _backgroundmusicaudio (`self.BackgroundMusicAudio` :!label _label)
        (:`then`
          (`AudioComponent.Stop` _backgroundmusicaudio)
          (`ActorComponent.K2_DestroyComponent` _backgroundmusicaudio)
          (set `self.BackgroundMusicAudio` null))
        (:`else`)))
    (:`then_1`
      (bind _returnvalue (`GameplayStatics.CreateSound2D` Sound 1.0 1.0 0.0 null))
      (bind _output_get (set `self.BackgroundMusicAudio` _returnvalue))
      (`AudioComponent.Play` _output_get 0.0))))

(event `UpdateBackgroundMusic`
  (bind _backgroundmusiccolls (`self.BackgroundMusicColls`))
  (bind _backgroundmusicaudio (`self.BackgroundMusicAudio`))
  (bind _returnvalue (`KismetArrayLibrary.Array_LastIndex` _backgroundmusiccolls))
  (bind _sound (`/Game/BackgroundMusicSystem/BP_BackgroundMusic.Sound` (`|GetArrayItem` _backgroundmusiccolls _returnvalue)))
  (if (== _returnvalue -1)
    (goto _label)
    (else
      (`/Engine/EditorBlueprintResources/StandardMacros.IsValid` _backgroundmusicaudio
        (:`Is Valid`
          (if (!= (`AudioComponent.Sound` _backgroundmusicaudio) _sound)
            (`self.PlayMusic` _sound :!label _label_2)))
        (:`Is Not Valid`
          (goto _label_2))))))

(fn `UserConstructionScript`)