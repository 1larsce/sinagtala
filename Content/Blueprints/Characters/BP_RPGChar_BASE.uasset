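; Base RPG character Blueprint that provides dialogue interaction driven by a DialogueTable data table.
; Interact locks both participants via StartInteraction, stops movement, shows the first line on the GM_RPG HUD dialogue widget and enables the mouse cursor.
; ShowNextLine steps through rows by index with a sound cue, returning false when none remain.
; FinishInteraction restores game-only input, resets the line index and releases this character's lock.
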(event `self.ReceiveBeginPlay`
  (`PrimitiveComponent.SetCastShadow` (`self.DialogueIndicator`) false)
  (bind _asgm_rpg (cast `/Game/Blueprints/GM_RPG` (`GameplayStatics.GetGameMode`)))
  (set `self.GameMode` _asgm_rpg))

(event `/Game/Blueprints/Interfaces/BPI_Interaction.Interact`
  (params (Instigator :type "/Game/Blueprints/Characters/BP_RPGChar_BASE Object Reference"))
  (bind _returnvalue (`GameplayStatics.GetPlayerController` 0))
  (bind _dialoguetable (`self.DialogueTable`))
  (`/Engine/EditorBlueprintResources/StandardMacros.IsValid` _dialoguetable
    (:`Is Valid`
      (bind _outrownames (`DataTableFunctionLibrary.GetDataTableRowNames` _dialoguetable))
      (if (`KismetArrayLibrary.Array_IsValidIndex` _outrownames (`self.DialogueLineID`))
        (`self.StartInteraction` Instigator null)
        (`self.StartInteraction` Instigator)
        (`self.ShowDialogueLine`)
        (`WidgetBlueprintLibrary.SetInputMode_GameAndUIEx` _returnvalue null "DoNotLock" true true)
        (set `PlayerController.bShowMouseCursor` true _returnvalue)))))

(event `/Game/Blueprints/Interfaces/BPI_Interaction.FinishInteraction`
  (bind _returnvalue (`GameplayStatics.GetPlayerController` 0))
  (`WidgetBlueprintLibrary.SetInputMode_GameOnly` _returnvalue)
  (set `PlayerController.bShowMouseCursor` false _returnvalue)
  (set `self.DialogueLineID` 0)
  (`self.EndInteraction`))

(fn `EndInteraction`
  (set `self.IsInteractionLocked` false))

(fn `ShowDialogueLine`
  (bind _dialoguetable (`self.DialogueTable`))
  (bind _dialoguelineid (`self.DialogueLineID`))
  (`/Engine/EditorBlueprintResources/StandardMacros.IsValid` _dialoguetable
    (:`Is Valid`
      (bind _outrownames (`DataTableFunctionLibrary.GetDataTableRowNames` _dialoguetable))
      (if (`KismetArrayLibrary.Array_IsValidIndex` _outrownames _dialoguelineid)
        (bind _returnvalue (`|GetDataTableRow` _dialoguetable (`|GetArrayItem` _outrownames _dialoguelineid))
          (:`then`
            (`/Game/DialogueSystem/WBP_Dialogue.ShowLine` (`/Game/Widgets/WBP_HUD.WBP_Dialogue` (`/Game/Blueprints/GM_RPG.HUDWidget` (`self.GameMode`))) _returnvalue)
            (`/Engine/EditorBlueprintResources/StandardMacros.IncrementInt` (`self.DialogueLineID`)
              (:`  `
                (return)))))))))

(fn `ShowNextLine`
  (returns (HasNextLine :type Boolean))
  (bind _dialoguetable (`self.DialogueTable`))
  (`/Engine/EditorBlueprintResources/StandardMacros.IsValid` _dialoguetable
    (:`Is Valid`
      (bind _outrownames (`DataTableFunctionLibrary.GetDataTableRowNames` _dialoguetable))
      (if (`KismetArrayLibrary.Array_IsValidIndex` _outrownames (`self.DialogueLineID`))
        (`self.ShowDialogueLine`)
        (`GameplayStatics.PlaySound2D` "/Game/Sounds/Ambience/S_Dialogue_Cue.S_Dialogue_Cue" 1.0 1.0 0.0 null null)
        (return true)
        (else
          _)))
    (:`Is Not Valid`
      _))
  (return false))

(fn `StartInteraction`
  (params (InteractInstigator :type "Actor Object Reference"))
  (set `self.IsInteractionLocked` true)
  (`MovementComponent.StopMovementImmediately` (`self.CharacterMovement`))
  (`GameplayStatics.PlaySound2D` "/Game/Sounds/Ambience/S_Dialogue_Cue.S_Dialogue_Cue" 1.0 1.0 0.0 null null))

(fn `UserConstructionScript`)