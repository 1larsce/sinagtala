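; BP_BackgroundMusic is a box trigger volume that tells GM_RPG when the player enters or leaves a background music area.
; Entering adds the volume to the game mode's BackgroundMusicColls and leaving removes it, each followed by UpdateBackgroundMusic.
; Two DoOnce gates reset each other, so enter and exit alternate without duplicate registrations.
; A next-tick check on BeginPlay covers a player who starts inside the box.
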(event `self.ReceiveBeginPlay`
  (bind _gamemoderef (`self.GameModeRef`))
  (bind _asgm_rpg (cast `/Game/Blueprints/GM_RPG` (`GameplayStatics.GetGameMode`)))
  (set `self.GameModeRef` _asgm_rpg)
  (`KismetSystemLibrary.DelayUntilNextTick`)
  (if (`KismetArrayLibrary.Array_Contains` (`PrimitiveComponent.GetOverlappingActors` (`self.Box`) null) (`GameplayStatics.GetPlayerCharacter` 0))
    (`/Engine/EditorBlueprintResources/StandardMacros.DoOnce` false :!label _label
      (:`Completed`
        (`|ExecutionSequence`
          (:`then_0`
            (`KismetArrayLibrary.Array_Add` (`/Game/Blueprints/GM_RPG.BackgroundMusicColls` _gamemoderef) self)
            (`/Game/Blueprints/GM_RPG.UpdateBackgroundMusic` _gamemoderef :!label _label_2))
          (:`then_1`
            (goto _label_3 :!via `Reset`)))))))

(event `self.Box.OnComponentBeginOverlap`
  (params (OverlappedComponent :type "PrimitiveComponent Object Reference") (OtherActor :type "Actor Object Reference") (OtherComp :type "PrimitiveComponent Object Reference") (OtherBodyIndex :type Integer) (bFromSweep :type Boolean) (SweepResult :type "HitResult Structure (by ref)"))
  (if (== OtherActor (`GameplayStatics.GetPlayerCharacter` 0))
    (goto _label)))

(event `self.Box.OnComponentEndOverlap`
  (params (OverlappedComponent :type "PrimitiveComponent Object Reference") (OtherActor :type "Actor Object Reference") (OtherComp :type "PrimitiveComponent Object Reference") (OtherBodyIndex :type Integer))
  (if (== OtherActor (`GameplayStatics.GetPlayerCharacter` 0))
    (`/Engine/EditorBlueprintResources/StandardMacros.DoOnce` false :!label _label_3
      (:`Completed`
        (`|ExecutionSequence`
          (:`then_0`
            (`KismetArrayLibrary.Array_RemoveItem` (`/Game/Blueprints/GM_RPG.BackgroundMusicColls` (`self.GameModeRef`)) self)
            (goto _label_2))
          (:`then_1`
            (goto _label :!via `Reset`)))))))

(fn `UserConstructionScript`)