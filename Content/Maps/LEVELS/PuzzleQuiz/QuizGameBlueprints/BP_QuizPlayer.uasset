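; BP_QuizPlayer is the player character for the PuzzleQuiz level, handling movement, jumping and sprinting through Enhanced Input.
; On BeginPlay it adds the IMC_Mazer mapping context to its player controller's input subsystem.
; IA_Maze moves the character along fixed world X and Y axes, independent of camera or control rotation.
; Sprint raises CharacterMovement's max walk speed while triggered and sets it back on completion.
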(event `EnhancedInput|/Game/Input/Actions/IA_Jump`
  (params (ActionValue :type Boolean) (ElapsedSeconds :type "Float (double-precision)") (TriggeredSeconds :type "Float (double-precision)") (InputAction :type "InputAction Object Reference" :default "/Game/Input/Actions/IA_Jump.IA_Jump"))
  ; Jump and Sprint
  (:`Started`
    (`self.Jump`))
  (:`Completed`
    (`self.StopJumping`)))

(event `EnhancedInput|/Game/Input/Actions/IA_Sprint`
  (params (ActionValue :type Boolean) (ElapsedSeconds :type "Float (double-precision)") (TriggeredSeconds :type "Float (double-precision)") (InputAction :type "InputAction Object Reference" :default "/Game/Input/Actions/IA_Sprint.IA_Sprint"))
  (bind _charactermovement (`self.CharacterMovement`))
  ; Jump and Sprint
  (:`Triggered`
    (set `CharacterMovementComponent.MaxWalkSpeed` 1500.0 _charactermovement))
  (:`Completed`
    (set `CharacterMovementComponent.MaxWalkSpeed` 1000.0 _charactermovement)))

(event `self.ReceiveBeginPlay`
  ; Movement
  (bind _asplayer_controller (cast `PlayerController` (`self.GetController`)))
  (`EnhancedInputSubsystemInterface.AddMappingContext` (pcsubsystem `EnhancedInputLocalPlayerSubsystem` _asplayer_controller) "/Game/Maps/LEVELS/Maze/Input/IMC_Mazer.IMC_Mazer" 0 (struct)))

(event `EnhancedInput|/Game/Maps/LEVELS/Maze/Input/IA_Maze`
  (params (ActionValue :type "Vector2D Structure") (ElapsedSeconds :type "Float (double-precision)") (TriggeredSeconds :type "Float (double-precision)") (InputAction :type "InputAction Object Reference" :default "/Game/Maps/LEVELS/Maze/Input/IA_Maze.IA_Maze"))
  (bind (_x _y) (`KismetMathLibrary.BreakVector2D` ActionValue))
  ; Movement
  (:`Triggered`
    (`self.AddMovementInput` (1.0 0.0 0.0) _x)
    (`self.AddMovementInput` (0.0 1.0 0.0) _y)))

(fn `UserConstructionScript`)