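; Player character for the puzzle quiz level, with sprite, minimap, movement, jump, sprint, dialogue and quest support.
; BeginPlay loads quests from the GameInstance save, and P writes them back to a slot.
; Tick feeds player position to a masking material parameter collection and sphere-traces for interactables, whose returned IDs advance quest objectives.
; A separate overlap-based interact starts and steps through HUD dialogue, skipping text reveal and blocking movement while locked.
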(event `self.ReceiveBeginPlay`
  (`parent.ReceiveBeginPlay`)
  (`|ExecutionSequence`
    (:`then_0`
      (bind _asplayer_controller (cast `PlayerController` (`self.GetController`)))
      (`EnhancedInputSubsystemInterface.AddMappingContext` (pcsubsystem `EnhancedInputLocalPlayerSubsystem` _asplayer_controller) "/Game/Input/IMC_RPG.IMC_RPG" 0 (struct))
      (bind _returnvalue (`|CreateWidget` "/Game/MiniMap/WB_MiniMap.WB_MiniMap_C" (`GameplayStatics.GetPlayerController` 0)))
      (`UserWidget.AddToViewport` _returnvalue 0))
    (:`then_1`
      (`PlayerController.SetAudioListenerOverride` (`GameplayStatics.GetPlayerController` 0) (`self.Sprite`) (0.0 0.0 0.0) (struct :`Yaw` 270.0)))
    (:`then_2`
      (bind _asmy_game_instance (cast `/Game/QuestSystem/MyGameInstance` (`GameplayStatics.GetGameInstance`)))
      (bind _output_get (set `self.As My Game Instance` _asmy_game_instance))
      (`/Game/QuestSystem/MySaveData.LoadQuests` (`/Game/QuestSystem/MyGameInstance.SaveData` _output_get) (`self.QuestLogComponent`)))))

(event `self.ReceiveTick`
  (params (DeltaSeconds :type "Float (single-precision)"))
  ; Masking
  (`parent.ReceiveTick` DeltaSeconds)
  (`KismetMaterialLibrary.SetVectorParameterValue` "/Game/Materials/MPC_Masking.MPC_Masking" "PlayerPosition" (`KismetMathLibrary.Conv_VectorToLinearColor` (`self.K2_GetActorLocation`)))
  (`self.InteractTrace`))

(event `EnhancedInput|/Game/Input/Actions/IA_QuestInteract`
  (params (ActionValue :type Boolean) (ElapsedSeconds :type "Float (double-precision)") (TriggeredSeconds :type "Float (double-precision)") (InputAction :type "InputAction Object Reference" :default "/Game/Input/Actions/IA_QuestInteract.IA_QuestInteract"))
  ; Part 3
  (:`Started`
    (bind _lookatactor (`self.LookAtActor`)
      (:`then`
        (bind _objectiveid (message `/Game/QuestSystem/Interact/IInteractionInterface.InteractWith` _lookatactor))
        (`self.OnObjectiveIDCalled` _objectiveid 1))
      (:`else`))))

(event `Key|P`
  (params (Key :type "Key Structure"))
  (bind _savedata (`/Game/QuestSystem/MyGameInstance.SaveData` (`self.As My Game Instance`)))
  ; Save Game
  (:`Pressed`
    (bind _asmy_game_instance (cast `/Game/QuestSystem/MyGameInstance` (`GameplayStatics.GetGameInstance`)))
    (set `self.As My Game Instance` _asmy_game_instance)
    (for _array_element (`/Game/QuestSystem/QuestLogComponent.CurrentQuests` (`self.QuestLogComponent`))
      (`/Game/QuestSystem/MySaveData.SaveQuestDetails` _savedata _array_element))
    (`/Game/QuestSystem/MySaveData.SaveQuestLog` _savedata (`self.QuestLogComponent`))
    (`GameplayStatics.SaveGameToSlot` (`/Game/QuestSystem/MyGameInstance.SaveData` (`self.As My Game Instance`)) "savedata")))

(event `EnhancedInput|/Game/Input/Actions/IA_Move`
  (params (ActionValue :type "Vector2D Structure") (ElapsedSeconds :type "Float (double-precision)") (TriggeredSeconds :type "Float (double-precision)") (InputAction :type "InputAction Object Reference" :default "/Game/Input/Actions/IA_Move.IA_Move"))
  (bind (_x _y) (`KismetMathLibrary.BreakVector2D` ActionValue))
  ; MOVE
  (:`Triggered`
    (if (not (`self.IsInteractionLocked`))
      (`self.AddMovementInput` (1.0 0.0 0.0) _x)
      (`self.AddMovementInput` (0.0 1.0 0.0) _y))))

(event `EnhancedInput|/Game/Input/Actions/IA_Jump`
  (params (ActionValue :type Boolean) (ElapsedSeconds :type "Float (double-precision)") (TriggeredSeconds :type "Float (double-precision)") (InputAction :type "InputAction Object Reference" :default "/Game/Input/Actions/IA_Jump.IA_Jump"))
  ; Jump and Sprint
  (:`Started`
    (`self.Jump`))
  (:`Completed`
    (`self.StopJumping`)))

(event `EnhancedInput|/Game/Input/Actions/IA_Sprint`
  (params (ActionValue :type Boolean) (ElapsedSeconds :type "Float (double-precision)") (TriggeredSeconds :type "Float (double-precision)") (InputAction :type "InputAction Object Reference" :default "/Game/Input/Actions/IA_Sprint.IA_Sprint"))
  (bind _charactermovement (`self.CharacterMovement`))
  ; Jump and Sprint
  (:`Triggered`
    (set `CharacterMovementComponent.MaxWalkSpeed` 1500.0 _charactermovement))
  (:`Completed`
    (set `CharacterMovementComponent.MaxWalkSpeed` 1000.0 _charactermovement)))

(event `OnChoiceSelect`
  (bind _returnvalue (`GameplayStatics.GetPlayerController` 0))
  (bind _wbp_dialogue (`/Game/Widgets/WBP_HUD.WBP_Dialogue` (`/Game/Blueprints/GM_RPG.HUDWidget` (`self.GameMode`))))
  ; IA_Interact
  (if (`self.IsInteractionLocked`) :!label _label
    (bind _returnvalue_2 (`/Game/DialogueSystem/WBP_Dialogue.IsFinishedRevealing` _wbp_dialogue))
    (if _returnvalue_2
      (bind _lastinteracted (`self.LastInteracted`)
        (:`then`
          (bind _hasnextline (message `/Game/Blueprints/Interfaces/BPI_Interaction.ShowNextLine` _lastinteracted))
          (if (not _hasnextline)
            (`self.EndInteraction`)
            (bind _lastinteracted_2 (`self.LastInteracted`)
              (:`then`
                (message `/Game/Blueprints/Interfaces/BPI_Interaction.FinishInteraction` _lastinteracted_2)
                (`/Game/Widgets/WBP_HUD.SetDialogueWidgetVisibility` (`/Game/Blueprints/GM_RPG.HUDWidget` (`self.GameMode`)) false)
                (`WidgetBlueprintLibrary.SetInputMode_GameOnly` _returnvalue)
                (set `PlayerController.bShowMouseCursor` false _returnvalue))
              (:`else`))))
        (:`else`))
      (else
        (`/Game/DialogueSystem/WBP_Dialogue.InstaReveal` _wbp_dialogue)))
    (else
      (for _array_element (`PrimitiveComponent.GetOverlappingActors` (`self.InteractionCheck`) null)
        (if (!= _array_element self)
          (message `/Game/Blueprints/Interfaces/BPI_Interaction.Interact` _array_element self)
          (set `self.LastInteracted` _array_element)
          (break))))))

(event `EnhancedInput|/Game/Input/Actions/IA_Interact`
  (params (ActionValue :type Boolean) (ElapsedSeconds :type "Float (double-precision)") (TriggeredSeconds :type "Float (double-precision)") (InputAction :type "InputAction Object Reference" :default "/Game/Input/Actions/IA_Interact.IA_Interact"))
  ; IA_Interact
  (:`Started`
    (goto _label)))

(fn `InteractTrace`
  (bind _returnvalue (`self.K2_GetActorLocation`))
  ; Part 3:
  (bind (_outhit _returnvalue_2) (`KismetSystemLibrary.SphereTraceSingle` _returnvalue (+ _returnvalue (* (`self.GetActorForwardVector`) 200.0)) 20.0 "TraceTypeQuery2" false (`|MakeArray` (`self.GetOwner`))))
  (if _returnvalue_2
    (bind (_bblockinghit _binitialoverlap _time _distance _location _impactpoint _normal _impactnormal _physmat _hitactor) (`GameplayStatics.BreakHitResult` _outhit))
    (if (`KismetSystemLibrary.DoesImplementInterface` _hitactor "/Game/QuestSystem/Interact/IInteractionInterface.IInteractionInterface_C")
      (bind _output_get (set `self.LookAtActor` _hitactor))
      (message `/Game/QuestSystem/Interact/IInteractionInterface.LookAt` _output_get)
      (else
        (set `self.LookAtActor` null)))
    (else
      (set `self.LookAtActor` null))))

(fn `UserConstructionScript`
  (`parent.UserConstructionScript`))