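; DP_Enter_BP is a trigger box in the puzzle quiz system that opens DP_Widget when BP_Player steps inside.
; On overlap it disables movement and look input, creates or reveals the cached widget, and switches to UI-only input with the cursor shown.
; When the overlap ends it restores walking and, if the widget exists, collapses it, restores game input and destroys itself, making the trigger single-use.
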(event `self.Box.OnComponentBeginOverlap`
  (params (OverlappedComponent :type "PrimitiveComponent Object Reference") (OtherActor :type "Actor Object Reference") (OtherComp :type "PrimitiveComponent Object Reference") (OtherBodyIndex :type Integer) (bFromSweep :type Boolean) (SweepResult :type "HitResult Structure (by ref)"))
  (bind _returnvalue (`GameplayStatics.GetPlayerController` 0))
  (bind _asbp_player (cast `/Game/Blueprints/Characters/BP_Player` OtherActor))
  (`CharacterMovementComponent.SetMovementMode` (`Character.CharacterMovement` _asbp_player) "MOVE_None" 0)
  (bind _widget_ref (`self.Widget Ref`)
    (:`then`
      (`Widget.SetVisibility` _widget_ref "Visible"))
    (:`else`
      (bind _returnvalue_2 (`|CreateWidget` "/Game/Maps/LEVELS/PuzzleQuiz/QuizSystem/Widgets/DP_Widget.DP_Widget_C" null _asbp_player))
      (bind _output_get (set `self.Widget Ref` _returnvalue_2))
      (`UserWidget.AddToViewport` _output_get 0)))
  (`Controller.SetIgnoreLookInput` _returnvalue true)
  (set `PlayerController.bShowMouseCursor` true _returnvalue)
  (`WidgetBlueprintLibrary.SetInputMode_UIOnlyEx` _returnvalue null))

(event `self.Box.OnComponentEndOverlap`
  (params (OverlappedComponent :type "PrimitiveComponent Object Reference") (OtherActor :type "Actor Object Reference") (OtherComp :type "PrimitiveComponent Object Reference") (OtherBodyIndex :type Integer))
  (bind _returnvalue (`GameplayStatics.GetPlayerController` 0))
  (bind _asbp_player (cast `/Game/Blueprints/Characters/BP_Player` OtherActor))
  (`CharacterMovementComponent.SetMovementMode` (`Character.CharacterMovement` _asbp_player) "MOVE_Walking" 0)
  (bind _widget_ref (`self.Widget Ref`)
    (:`then`
      (`Widget.SetVisibility` _widget_ref "Collapsed")
      (`Controller.ResetIgnoreLookInput` _returnvalue)
      (`WidgetBlueprintLibrary.SetInputMode_GameOnly` _returnvalue)
      (set `PlayerController.bShowMouseCursor` false _returnvalue)
      (`self.K2_DestroyActor`))
    (:`else`)))

(fn `UserConstructionScript`)