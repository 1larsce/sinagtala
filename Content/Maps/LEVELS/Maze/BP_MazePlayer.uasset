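; Player pawn for the Maze level, handling movement, a spectator free cam, pausing and interaction.
; Enhanced Input adds IMC_Mazer on BeginPlay and drives movement along fixed world X/Y axes rather than camera-relative ones.
; Spectator input spawns and possesses BP_SpectatorCamera at the camera's transform, while pause input toggles a cached WB_Pause, game pause, cursor and input mode.
; A hard-bound E key sphere-traces forward and sends NoteInteractionMessage to the hit actor.
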(event `self.ReceiveBeginPlay`
  ; Movement
  (bind _asplayer_controller (cast `PlayerController` (`self.GetController`)))
  (`EnhancedInputSubsystemInterface.AddMappingContext` (pcsubsystem `EnhancedInputLocalPlayerSubsystem` _asplayer_controller) "/Game/Maps/LEVELS/Maze/Input/IMC_Mazer.IMC_Mazer" 0 (struct)))

(event `EnhancedInput|/Game/Maps/LEVELS/Maze/Input/IA_Maze`
  (params (ActionValue :type "Vector2D Structure") (ElapsedSeconds :type "Float (double-precision)") (TriggeredSeconds :type "Float (double-precision)") (InputAction :type "InputAction Object Reference" :default "/Game/Maps/LEVELS/Maze/Input/IA_Maze.IA_Maze"))
  (bind (_x _y) (`KismetMathLibrary.BreakVector2D` ActionValue))
  ; Movement
  (:`Triggered`
    (`self.AddMovementInput` (1.0 0.0 0.0) _x)
    (`self.AddMovementInput` (0.0 1.0 0.0) _y)))

(event `EnhancedInput|/Game/Maps/LEVELS/Maze/Input/IA_Spectator`
  (params (ActionValue :type Boolean) (ElapsedSeconds :type "Float (double-precision)") (TriggeredSeconds :type "Float (double-precision)") (InputAction :type "InputAction Object Reference" :default "/Game/Maps/LEVELS/Maze/Input/IA_Spectator.IA_Spectator"))
  ; Spectator Free Cam
  (:`Started`
    (bind _returnvalue (`|SpawnActorFromClass` "/Game/Maps/LEVELS/Maze/BP_SpectatorCamera.BP_SpectatorCamera_C" (`SceneComponent.K2_GetComponentToWorld` (`self.Camera`)) "AdjustIfPossibleButAlwaysSpawn" "MultiplyWithRoot" null null))
    (`Controller.Possess` (`GameplayStatics.GetPlayerController` 0) _returnvalue)))

(event `EnhancedInput|/Game/Maps/LEVELS/Maze/Input/IA_Pause`
  (params (ActionValue :type Boolean) (ElapsedSeconds :type "Float (double-precision)") (TriggeredSeconds :type "Float (double-precision)") (InputAction :type "InputAction Object Reference" :default "/Game/Maps/LEVELS/Maze/Input/IA_Pause.IA_Pause"))
  (bind _returnvalue (`GameplayStatics.GetPlayerController` 0))
  (bind _returnvalue_2 (`GameplayStatics.GetPlayerController` 0))
  (bind _pauseref (`self.PauseRef`))
  ; Pause Game
  (:`Started`
    (`/Engine/EditorBlueprintResources/StandardMacros.IsValid` (`self.PauseRef`)
      (:`Is Valid`
        _)
      (:`Is Not Valid`
        (bind _returnvalue_3 (`|CreateWidget` "/Game/EasyParallaxMenu/WidgetsMain/WB_Pause.WB_Pause_C"))
        (set `self.PauseRef` _returnvalue_3)))
    (if (`GameplayStatics.IsGamePaused`)
      (`Widget.RemoveFromParent` (`self.PauseRef`))
      (`GameplayStatics.SetGamePaused` false)
      (set `PlayerController.bShowMouseCursor` false _returnvalue_2)
      (`WidgetBlueprintLibrary.SetInputMode_GameOnly` _returnvalue_2)
      (else
        (`UserWidget.AddToViewport` _pauseref 0)
        (`GameplayStatics.SetGamePaused` true)
        (set `PlayerController.bShowMouseCursor` true _returnvalue)
        (`WidgetBlueprintLibrary.SetInputMode_GameAndUIEx` _returnvalue _pauseref)))))

(event `Key|E`
  (params (Key :type "Key Structure"))
  (bind _returnvalue (`self.K2_GetActorLocation`))
  ; Interaction(General)
  (:`Pressed`
    (bind (_outhit _returnvalue_2) (`KismetSystemLibrary.SphereTraceSingle` _returnvalue (+ _returnvalue (* (`self.GetActorForwardVector`) 200.0)) 100.0 "TraceTypeQuery2" false (`|MakeArray` (`self.GetOwner`))))
    (if _returnvalue_2
      (message `/Game/Maps/LEVELS/Maze/Reusablepics/NoteInteraction_Interface.NoteInteraction` (`.HitActor` (`GameplayStatics.BreakHitResult` _outhit))))))

(fn `UserConstructionScript`)