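; Actor component that lets its owner detect, interact with and inspect objects in front of it.
; A looping timer replaces Tick, running a short forward sphere trace for actors implementing BPI_ObjectInteraction.
; The hit actor becomes the target and supplies look-at text to an on-screen WB_InteractMessage widget, cleared otherwise.
; Enhanced Input actions send interact or inspect calls to the target; inspecting also removes the widget from screen.
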(event `self.ReceiveBeginPlay`
  (`self.CreateInteractMessage`)
  (`self.BeginInteraction`))

(event `BeginInteraction`
  (`KismetSystemLibrary.K2_SetTimerDelegate` (delegate `UpdateInteraction`) 0.2 true))

(event `UpdateInteraction`
  (`self.CapsuleTrace`))

(event `EnhancedInput|/Game/Maps/LEVELS/Maze/Input/IA_ObjectInteract`
  (params (ActionValue :type Boolean) (ElapsedSeconds :type "Float (double-precision)") (TriggeredSeconds :type "Float (double-precision)") (InputAction :type "InputAction Object Reference" :default "/Game/Maps/LEVELS/Maze/Input/IA_ObjectInteract.IA_ObjectInteract"))
  (:`Started`
    (bind _targetactor (`self.TargetActor`)
      (:`then`
        (message `/Game/Maps/LEVELS/Maze/ObjectInteraction/BPI_ObjectInteraction.ObjectInteractWith` _targetactor (`/Game/Maps/LEVELS/Maze/BP_UniversalLibrary.GetMyPlayer`))
        (`KismetSystemLibrary.PrintString` "Interacting"))
      (:`else`))))

(event `EnhancedInput|/Game/Maps/LEVELS/Maze/Input/IA_Inspect`
  (params (ActionValue :type Boolean) (ElapsedSeconds :type "Float (double-precision)") (TriggeredSeconds :type "Float (double-precision)") (InputAction :type "InputAction Object Reference" :default "/Game/Maps/LEVELS/Maze/Input/IA_Inspect.IA_Inspect"))
  (:`Started`
    (bind _targetactor (`self.TargetActor`)
      (:`then`
        (message `/Game/Maps/LEVELS/Maze/ObjectInteraction/BPI_ObjectInteraction.Inspect` _targetactor (struct))
        (`KismetSystemLibrary.PrintString` "Inspecting")
        (`Widget.RemoveFromParent` (`self.WB_InteractMessage`)))
      (:`else`))))

(fn `CapsuleTrace`
  (bind _returnvalue (`self.GetOwner`))
  (bind _returnvalue_2 (`Actor.K2_GetActorLocation` _returnvalue))
  (bind (_outhit _returnvalue_3) (`KismetSystemLibrary.SphereTraceSingle` _returnvalue_2 (+ _returnvalue_2 (* (`Actor.GetActorForwardVector` _returnvalue) 150.0)) 0.0 "TraceTypeQuery3"))
  (if _returnvalue_3
    (bind (_bblockinghit _binitialoverlap _time _distance _location _impactpoint _normal _impactnormal _physmat _hitactor) (`GameplayStatics.BreakHitResult` _outhit))
    (if (`KismetSystemLibrary.DoesImplementInterface` _hitactor "/Game/Maps/LEVELS/Maze/ObjectInteraction/BPI_ObjectInteraction.BPI_ObjectInteraction_C")
      (bind _output_get (set `self.TargetActor` _hitactor))
      (bind _message (message `/Game/Maps/LEVELS/Maze/ObjectInteraction/BPI_ObjectInteraction.LookAt` _output_get))
      (`/Game/Maps/LEVELS/Maze/ObjectInteraction/UI/WB_InteractMessage.SetMessage` (`self.WB_InteractMessage`) _message)
      (else
        (set `self.TargetActor` null)
        (`/Game/Maps/LEVELS/Maze/ObjectInteraction/UI/WB_InteractMessage.SetMessage` (`self.WB_InteractMessage`) "")))
    (else
      (set `self.TargetActor` null)
      (`/Game/Maps/LEVELS/Maze/ObjectInteraction/UI/WB_InteractMessage.SetMessage` (`self.WB_InteractMessage`) ""))))

(fn `CreateInteractMessage`
  (bind _returnvalue (`|CreateWidget` "/Game/Maps/LEVELS/Maze/ObjectInteraction/UI/WB_InteractMessage.WB_InteractMessage_C"))
  (bind _output_get (set `self.WB_InteractMessage` _returnvalue))
  (`UserWidget.AddToViewport` _output_get 0))