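; BP_NPC_NavMesh1 is a NavMesh-driven NPC that wanders until it sees the player, then chases them.
; Pawn sensing stores the player and sets a seeing flag, which a retriggerable delay clears shortly after sightings stop.
; Tick uses DoOnce gates to pick random reachable wander points periodically or issue an AI MoveTo on the player.
; Reaching the player calls its Lose function, while a failed chase re-arms the gate.
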(event `MoveNPC`
  (bind _output_get (set `self.Random Location` (`NavigationSystemV1.K2_GetRandomReachablePointInRadius` (`self.K2_GetActorLocation`) 1000.0 null null)))
  (`|AIMoveTo` self _output_get null))

(event `self.PawnSensing.OnSeePawn`
  (params (Pawn :type "Pawn Object Reference"))
  (bind _asbp_player_run_1 (cast `/Game/Maps/LEVELS/Run/Blueprints/BP_PlayerRun1` Pawn))
  (set `self.PlayerFollowed` _asbp_player_run_1)
  (`|ExecutionSequence`
    (:`then_0`
      (set `self.Seeing Player` true))
    (:`then_1`
      (`KismetSystemLibrary.RetriggerableDelay` 0.6)
      (set `self.Seeing Player` false))))

(event `self.ReceiveTick`
  (params (DeltaSeconds :type "Float (single-precision)"))
  (if (`self.Seeing Player`)
    (`/Engine/EditorBlueprintResources/StandardMacros.DoOnce` false :!label _label
      (:`Completed`
        (`|AIMoveTo` self (0.0 0.0 0.0) (`self.PlayerFollowed`) 250.0
          (:`OnSuccess`
            (`/Game/Maps/LEVELS/Run/Blueprints/BP_PlayerRun1.Lose` (`self.PlayerFollowed`)))
          (:`OnFail`
            (goto _label :!via `Reset`)))))
    (else
      (`/Engine/EditorBlueprintResources/StandardMacros.DoOnce` false :!label _label_2
        (:`Completed`
          (`self.MoveNPC`)
          (`KismetSystemLibrary.Delay` 4.0)
          (goto _label_2 :!via `Reset`))))))

(fn `UserConstructionScript`)