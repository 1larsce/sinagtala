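; Game mode for the Run minigame level that holds the player still through a pre-start countdown.
; On BeginPlay it shows the WB_Countdown widget, disables the player character's input and starts a looping one-second timer.
; Each tick of that timer decrements Count, updates the widget text and plays a notification sound.
; At zero it clears the timer, removes the widget and re-enables input.
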(event `self.ReceiveBeginPlay`
  (bind _returnvalue (`|CreateWidget` "/Game/Maps/LEVELS/Run/Widget/WB_Countdown.WB_Countdown_C"))
  (bind _output_get (set `self.Countdown Widget` _returnvalue))
  (`UserWidget.AddToViewport` _output_get 0)
  (bind _returnvalue_2 (`KismetSystemLibrary.K2_SetTimerDelegate` (delegate `Take Countdown`) 1.0 true))
  (`self.DisableInput` (`GameplayStatics.GetPlayerCharacter` 0) (`GameplayStatics.GetPlayerController` 0)))

(event `Take Countdown`
  (`/Engine/EditorBlueprintResources/StandardMacros.DecrementInt` (`self.Count`)
    (:`  `
      (`TextBlock.SetText` (`/Game/Maps/LEVELS/Run/Widget/WB_Countdown.CountdownText` (`self.Countdown Widget`)) (`KismetTextLibrary.Conv_IntToText` (`self.Count`)))
      (`GameplayStatics.PlaySound2D` "/Game/Sounds/SFX/notif.notif" 1.0 1.0 0.0 null null)
      (if (<= (`self.Count`) 0)
        (`KismetSystemLibrary.K2_ClearAndInvalidateTimerHandle` (stale `self.ReceiveBeginPlay` _returnvalue_2))
        (`Widget.RemoveFromParent` (`self.Countdown Widget`))
        (`self.EnableInput` (`GameplayStatics.GetPlayerCharacter` 0) (`GameplayStatics.GetPlayerController` 0))))))

(fn `UserConstructionScript`)